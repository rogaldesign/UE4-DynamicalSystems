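; IK_Game_Mode is the game mode of the FullBodyIK content, customizing how players get their start point.
; Its FindPlayerStart override returns the PlayerStart whose tag matches the incoming name.
; Without a match it uses the first PlayerStart found, or spawns one at the world origin tagged "Spawned" when the level has none.
; BeginPlay, Tick and the construction script are empty.
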(event EventBeginPlay)

(event EventTick
  (params (DeltaSeconds :type Float%20%28single-precision%29)))

(fn ConstructionScript)

(fn FindPlayerStart
  (params (Player :type Controller%20Object%20Reference) (IncomingName :type String))
  (bind _outactors (Actor|GetAllActorsOfClass "/Script/Engine.PlayerStart"))
  (for _array_element _outactors
    (if (Utilities|Enum|Equal(Enum) IncomingName (Utilities|String|ToString(Name) (Variables|/Script/Engine.PlayerStart|GetPlayerStartTag _array_element)))
      (return _array_element)))
  (if (> (Utilities|Array|Length _outactors) 0)
    (return (Utilities|Array|Get(acopy) _outactors))
    (else
      (bind _returnvalue (Game|SpawnActorfromClass "/Script/Engine.PlayerStart" (Math|Transform|MakeTransform "0, 0, 0") "AlwaysSpawn" 0 0))
      (Variables|/Script/Engine.PlayerStart|SetPlayerStartTag _returnvalue "Spawned")
      (return _returnvalue))))