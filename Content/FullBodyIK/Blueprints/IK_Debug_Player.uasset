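; Debug player controller for full-body IK that spawns an IK pawn and camera at the first PlayerStart and possesses the pawn.
; Each tick drives the pawn's HMD and two motion controllers along sine/cosine circles, simulating tracked movement relative to height and floor.
; FloorNav traces downward and interpolates the pawn onto the ground, using Gravity-based speed for descents and preserving the camera's vertical offset.
; PageDown sets a fixed pawn height.
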(event EventBeginPlay
  (bind _outactors (Actor|GetAllActorsOfClass "/Script/Engine.PlayerStart"))
  (if (> (Utilities|Array|Length _outactors) 0)
    (bind _returnvalue (Game|SpawnActorfromClass "/DynamicalSystems/FullBodyIK/Blueprints/IK_Pawn.IK_Pawn_C" (Math|Transform|ComposeTransforms (Math|Transform|MakeTransform "0, 0, 0" "0,-90.000000, 0") (Transformation|GetActorTransform (Utilities|Array|Get(acopy) _outactors))) "AlwaysSpawn" 0 0))
    (bind _output_get (Variables|Default|SetIK_Pawn _returnvalue))
    (bind _returnvalue_2 (Game|SpawnActorfromClass "/DynamicalSystems/FullBodyIK/Blueprints/IK_Camera.IK_Camera_C" (Math|Transform|ComposeTransforms (Math|Transform|MakeTransform "0, 0, 0" "0,-90.000000, 0") (Transformation|GetActorTransform (Utilities|Array|Get(acopy) _outactors))) "AlwaysSpawn" 0 0))
    (Variables|Default|SetIK_Camera _returnvalue_2)
    (Actor|SetOwner (Variables|/Script/Engine.ChildActorComponent|GetChildActor (Variables|/DynamicalSystems/FullBodyIK/Blueprints/IK_Pawn.IK_Pawn_C|GetChildHMD (Variables|Default|GetIK_Pawn))) (Variables|Default|GetIK_Camera))
    (Pawn|Possess self (Variables|Default|GetIK_Pawn))))

(event EventTick
  (params (DeltaSeconds :type Float%20%28single-precision%29))
  (Utilities|IsValid (Variables|Default|GetIK_Pawn)
    (:Is%20Valid
      (Utilities|FlowControl|Sequence
        (:then_0
          (CallFunction|TestHandL))
        (:then_1
          (CallFunction|TestHandR))
        (:then_2
          (CallFunction|TestHMD))
        (:then_3
          (CallFunction|FloorNav DeltaSeconds))))))

(event Input|KeyboardEvents|PageDown
  (params (Key :type Key%20Structure))
  (:Released
    (Variables|/DynamicalSystems/FullBodyIK/Blueprints/IK_Pawn.IK_Pawn_C|SetHeight (Variables|Default|GetIK_Pawn) 5e+01)
    (Development|PrintString "Hello")))

(fn ConstructionScript)

(fn TestHandL
  (bind _returnvalue (Utilities|Time|GetGameTimeinSeconds))
  (bind _ik_pawn (Variables|Default|GetIK_Pawn))
  (bind _returnvalue_2 (* _returnvalue 1.8e+02))
  (Transformation|SetWorldLocation (Variables|/DynamicalSystems/FullBodyIK/Blueprints/IK_Pawn.IK_Pawn_C|GetChildMotionControllerL (Variables|Default|GetIK_Pawn)) (+ (* (Math|Vector|MakeVector 0.0 (Math|Trig|Cos(Degrees) _returnvalue_2) (Math|Trig|Sin(Degrees) _returnvalue_2)) 1e+01) (Math|Vector|MakeVector 6e+01 0.0 (+ (Variables|/DynamicalSystems/FullBodyIK/Blueprints/IK_Pawn.IK_Pawn_C|GetHeight _ik_pawn) (Variables|/DynamicalSystems/FullBodyIK/Blueprints/IK_Pawn.IK_Pawn_C|GetFloor _ik_pawn)))) false false))

(fn TestHandR
  (bind _returnvalue (Utilities|Time|GetGameTimeinSeconds))
  (bind _ik_pawn (Variables|Default|GetIK_Pawn))
  (bind _returnvalue_2 (* _returnvalue 1e+02))
  (Transformation|SetWorldLocation (Variables|/DynamicalSystems/FullBodyIK/Blueprints/IK_Pawn.IK_Pawn_C|GetChildMotionControllerR (Variables|Default|GetIK_Pawn)) (+ (* (Math|Vector|MakeVector (Math|Trig|Sin(Degrees) _returnvalue_2) 0.0 (Math|Trig|Cos(Degrees) _returnvalue_2)) 1e+01) (Math|Vector|MakeVector -3e+01 2e+01 (+ (Variables|/DynamicalSystems/FullBodyIK/Blueprints/IK_Pawn.IK_Pawn_C|GetHeight _ik_pawn) (Variables|/DynamicalSystems/FullBodyIK/Blueprints/IK_Pawn.IK_Pawn_C|GetFloor _ik_pawn)))) false false))

(fn TestHMD
  (bind _returnvalue (Utilities|Time|GetGameTimeinSeconds))
  (bind _ik_pawn (Variables|Default|GetIK_Pawn))
  (bind _returnvalue_2 (* _returnvalue 4e+01))
  (Transformation|SetWorldLocation (Variables|/DynamicalSystems/FullBodyIK/Blueprints/IK_Pawn.IK_Pawn_C|GetChildHMD (Variables|Default|GetIK_Pawn)) (+ (* (Math|Vector|MakeVector (Math|Trig|Sin(Degrees) _returnvalue_2) (Math|Trig|Cos(Degrees) _returnvalue_2) 0.0) 5e+01) (Math|Vector|MakeVector 0.0 2e+01 (+ (Variables|/DynamicalSystems/FullBodyIK/Blueprints/IK_Pawn.IK_Pawn_C|GetHeight _ik_pawn) (Variables|/DynamicalSystems/FullBodyIK/Blueprints/IK_Pawn.IK_Pawn_C|GetFloor _ik_pawn)))) false false))

(fn FloorNav
  (params (DeltaTime :type Float%20%28single-precision%29))
  (bind _ik_pawn (Variables|Default|GetIK_Pawn))
  (bind _ik_pawn_2 (Variables|Default|GetIK_Pawn))
  (bind _ik_camera (Variables|Default|GetIK_Camera))
  (bind _defaultsceneroot (Variables|/DynamicalSystems/FullBodyIK/Blueprints/IK_Camera.IK_Camera_C|GetDefaultSceneRoot _ik_camera))
  (bind _defaultsceneroot_2 (Variables|/DynamicalSystems/FullBodyIK/Blueprints/IK_Pawn.IK_Pawn_C|GetDefaultSceneRoot _ik_pawn))
  (bind _defaultsceneroot_3 (Variables|/DynamicalSystems/FullBodyIK/Blueprints/IK_Pawn.IK_Pawn_C|GetDefaultSceneRoot _ik_pawn_2))
  (bind _returnvalue (Transformation|GetWorldLocation _defaultsceneroot_3))
  (bind _returnvalue_2 (Transformation|GetWorldLocation _defaultsceneroot_2))
  (bind _returnvalue_3 (Transformation|GetWorldLocation _defaultsceneroot))
  (bind (_x _y _z) (Math|Vector|BreakVector _returnvalue_2))
  (LocalVariables|SetHeadOffset (- (.z (Transformation|GetWorldLocation (Variables|/DynamicalSystems/FullBodyIK/Blueprints/IK_Camera.IK_Camera_C|GetDefaultSceneRoot (Variables|Default|GetIK_Camera)))) _z))
  (bind (_outhit _returnvalue_4) (Collision|LineTraceByChannel (Math|Vector|MakeVector _x _y (+ _z 1e+02)) (Math|Vector|MakeVector _x _y (+ _z -2e+04)) "TraceTypeQuery1" false (Utilities|Array|MakeArray (Variables|Default|GetIK_Pawn)) "None" true "(R=1.000000,G=0.000000,B=0.000000,A=1.000000)" "(R=0.000000,G=1.000000,B=0.000000,A=1.000000)" 1.0))
  (if _returnvalue_4
    (Transformation|SetWorldLocation (Variables|/DynamicalSystems/FullBodyIK/Blueprints/IK_Pawn.IK_Pawn_C|GetDefaultSceneRoot (Variables|Default|GetIK_Pawn)) (Math|Interpolation|VInterpTo _returnvalue (.Location (Collision|BreakHitResult _outhit)) DeltaTime (Math|Float|MapRangeUnclamped (Math|Vector|DotProduct (Math|Vector|Normalize (- (.Location (Collision|BreakHitResult _outhit)) _returnvalue)) "0, 0,1.000000") 1.0 -1.0 1e+01 (Variables|Default|GetGravity))) false false)
    (bind _output_get (Variables|/DynamicalSystems/FullBodyIK/Blueprints/IK_Pawn.IK_Pawn_C|SetFloor (Variables|Default|GetIK_Pawn) (.Z (Math|Vector|BreakVector (Math|Interpolation|VInterpTo _returnvalue (.Location (Collision|BreakHitResult _outhit)) DeltaTime (Math|Float|MapRangeUnclamped (Math|Vector|DotProduct (Math|Vector|Normalize (- (.Location (Collision|BreakHitResult _outhit)) _returnvalue)) "0, 0,1.000000") 1.0 -1.0 1e+01 (Variables|Default|GetGravity)))))))
    (Transformation|SetWorldLocation _defaultsceneroot (Math|Vector|MakeVector (.x _returnvalue_3) (.y _returnvalue_3) (+ (LocalVariables|GetHeadOffset) (.z (Transformation|GetWorldLocation (Variables|/DynamicalSystems/FullBodyIK/Blueprints/IK_Pawn.IK_Pawn_C|GetDefaultSceneRoot (Variables|Default|GetIK_Pawn)))))) false false)))