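; NetAvatarSpawner spawns IK_Net_Player actors as network avatars for IDs the NetClient reports missing.
; Each Tick it checks MissingAvatar, spawns a player, gives its NetAvatar component that ID and the client, then clears the value.
; A DebugRemote option, off in Tick, instead keeps one debug player using the client's own avatar ID.
; The voice activity handler is bound on BeginPlay but does nothing.
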(event Custom|OnVoiceActivityMsg_Event_0
  (params (NetId :type Integer) (Value :type Float%20%28single-precision%29)))

(event Custom|SpawnNetPlayer
  (params (Client :type Net%20Client%20Object%20Reference) (DebugRemote :type Boolean))
  (if (select DebugRemote (not (Utilities|IsValid (Variables|Default|Getdebugplayer))) (>= (Variables|/Script/DynamicalSystems.NetClient|GetMissingAvatar Client) 0))
    (bind _returnvalue (Game|SpawnActorfromClass "/DynamicalSystems/FullBodyIK/Blueprints/IK_Net_Player.IK_Net_Player_C" (Math|Transform|MakeTransform "0, 0, 0" "0, 0, 0" "1,1,1") "AlwaysSpawn" 0 0))
    (bind _output_get (Variables|Default|Setdebugplayer _returnvalue))
    (Variables|/Script/DynamicalSystems.NetAvatar|SetNetID (Actor|GetComponentbyClass _output_get "/Script/DynamicalSystems.NetAvatar") (select DebugRemote (Variables|/Script/DynamicalSystems.NetAvatar|GetNetID (Variables|/Script/DynamicalSystems.NetClient|GetAvatar (Variables|Default|GetNetClient))) (Variables|/Script/DynamicalSystems.NetClient|GetMissingAvatar Client)))
    (Variables|/Script/DynamicalSystems.NetAvatar|SetNetClient (Actor|GetComponentbyClass _output_get "/Script/DynamicalSystems.NetAvatar") Client)
    (Variables|/Script/DynamicalSystems.NetClient|SetMissingAvatar Client -1)))

(event EventBeginPlay
  (EventDispatchers|AssignOnVoiceActivityMsg (Variables|Default|GetNetClient) (delegate Custom|OnVoiceActivityMsg_Event_0)))

(event Collision|EventActorBeginOverlap
  (params (OtherActor :type Actor%20Object%20Reference)))

(event EventTick
  (params (DeltaSeconds :type Float%20%28single-precision%29))
  (CallFunction|SpawnNetPlayer (Variables|Default|GetNetClient) false))

(fn ConstructionScript)