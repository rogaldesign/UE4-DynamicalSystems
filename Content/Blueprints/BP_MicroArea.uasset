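; BP_MicroArea is an interactable VR area that teleports the player to an offset location inside it, optionally shrunk.
; Hovering toggles a spawned hint bubble showing the world name.
; Interacting or EnterMicroArea teleports the player if none is inside, then disables the collider, which construction creates unless a custom one is used.
; ExitMicroArea clears the occupant and restores query collision; its return teleport is disconnected.
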(event OnHovered(BP_Interactable)
  (params (Selector :type BP%20Interactable%20Selector%20Object%20Reference))
  (CallFunction|ToggleBubble true (Variables|/Script/Engine.Actor|GetRootComponent (Default|GetPlayer Selector))))

(event OnUnhovered(BP_Interactable)
  (params (Selector :type BP%20Interactable%20Selector%20Object%20Reference))
  (CallFunction|ToggleBubble false))

(event OnInteracted(BP_Interactable)
  (params (Selector :type BP%20Interactable%20Selector%20Object%20Reference))
  (Utilities|IsPlayerInside
    (:False
      (Variables|Default|SetPlayerInside (stale Custom|EnterMicroArea _asik_vr_player))
      (bind _location (CallFunction|PickTeleportLocation))
      (Default|Teleportto (stale Custom|EnterMicroArea _asik_vr_player) _location "0, 0, 0" (Variables|Default|GetShrinkPlayer))
      (Collision|SetCollisionEnabled (Variables|Default|GetCollider) "NoCollision")
      (Variables|Default|SetOriginalPlayerLocation (Transformation|GetWorldLocation (Variables|/DynamicalSystems/FullBodyIK/Blueprints/IK_Camera.IK_Camera_C|GetDefaultSceneRoot (Variables|/DynamicalSystems/FullBodyIK/Blueprints/IK_VR_Player.IK_VR_Player_C|GetIK_Camera (stale Custom|EnterMicroArea _asik_vr_player))))))))

(event Custom|EnterMicroArea
  (bind _asik_vr_player (Utilities|Casting|CastToIK_VR_Player (Game|GetPlayerController 0)))
  (Utilities|IsPlayerInside
    (:False
      (Variables|Default|SetPlayerInside _asik_vr_player)
      (bind _location (CallFunction|PickTeleportLocation))
      (Default|Teleportto _asik_vr_player _location "0, 0, 0" (Variables|Default|GetShrinkPlayer))
      (Collision|SetCollisionEnabled (Variables|Default|GetCollider) "NoCollision")
      (Variables|Default|SetOriginalPlayerLocation (Transformation|GetWorldLocation (Variables|/DynamicalSystems/FullBodyIK/Blueprints/IK_Camera.IK_Camera_C|GetDefaultSceneRoot (Variables|/DynamicalSystems/FullBodyIK/Blueprints/IK_VR_Player.IK_VR_Player_C|GetIK_Camera _asik_vr_player)))))))

(event Custom|ExitMicroArea
  (Variables|Default|SetPlayerInside 0)
  (Collision|SetCollisionEnabled (Variables|Default|GetCollider) "QueryOnly"))

(event Custom|OnMiroWorldExit)

(event EventBeginPlay)

(fn ConstructionScript
  (if (not (Variables|Collision|GetUseCustomCollision))
    (bind _returnvalue (AddComponent|AddBoxComponent false (Math|Transform|MakeTransform "0, 0, 0")))
    (bind _output_get (Variables|Default|SetCollider _returnvalue))
    (Components|Box|SetBoxExtent _output_get (Variables|Collision|GetColliderExtents) true)
    (Collision|SetCollisionObjectType _output_get "ECC_GameTraceChannel2")))

(fn PickTeleportLocation
  (return (+ (Transformation|GetActorLocation) (Variables|Default|GetTeleportationLocation))))

(fn ToggleBubble
  (params (On :type Boolean) (LookAt :type Scene%20Component%20Object%20Reference))
  (bind _collider (Variables|Default|GetCollider))
  (if On
    (Utilities|IsValid (Variables|Default|GetNameBubble)
      (:Is%20Not%20Valid
        (bind _returnvalue (Game|SpawnActorfromClass "/DynamicalSystems/Blueprints/BP_HintBubble.BP_HintBubble_C" (Math|Transform|MakeTransform (+ (Math|Vector|MakeVector 0.0 0.0 (.Z (Math|Vector|BreakVector (* (Variables|/Script/Engine.BoxComponent|GetBoxExtent _collider) 0.5)))) (Transformation|GetWorldLocation _collider))) "Undefined" 0 LookAt (Variables|Default|GetWorld%20Name) 0))
        (Variables|Default|SetNameBubble _returnvalue)))
    (else
      (Utilities|IsValid (Variables|Default|GetNameBubble)
        (:Is%20Valid
          (Actor|DestroyActor (Variables|Default|GetNameBubble)))))))