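; Selector actor that detects interactable objects along its forward vector and lets the VR player interact with the hovered one.
; A looping timer drives periodic object line traces that ignore the IK VR player, its pawn and its camera.
; Hits with a BP_Interactable component update the cached hover target, sending hover and unhover notifications, while misses clear it.
; TryInteraction calls Interact on the cached component, passing itself as the source.
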(event Custom|PerformSampling
  (bind _returnvalue (Transformation|GetActorLocation))
  (bind _controller (CallFunction|GetPlayer))
  (bind (_outhit _returnvalue_2) (Collision|LineTraceForObjects _returnvalue (+ _returnvalue (* (Transformation|GetActorForwardVector) (Variables|Sampling|GetSample%20Distance))) (Utilities|Array|MakeArray (Variables|Default|GetTrace%20For%20Objects)) false (Utilities|Array|MakeArray _controller (Variables|/DynamicalSystems/FullBodyIK/Blueprints/IK_VR_Player.IK_VR_Player_C|GetIK_Pawn _controller) (Variables|/DynamicalSystems/FullBodyIK/Blueprints/IK_VR_Player.IK_VR_Player_C|GetIK_Camera _controller)) "None" true "(R=1.000000,G=0.000000,B=0.000000,A=1.000000)" "(R=0.000000,G=1.000000,B=0.000000,A=1.000000)" (Variables|Sampling|GetSampleRate)))
  (CallFunction|OnTraceHiResultt _returnvalue_2 _outhit))

(event Custom|OnTraceHiResultt
  (params (IsHit :type Boolean) (Result :type Hit%20Result%20Structure))
  (bind _hitactor (Collision|BreakHitResult Result))
  (bind _returnvalue (Actor|GetComponentbyClass _hitactor "/DynamicalSystems/Blueprints/ActorComponents/BP_Interactable.BP_Interactable_C"))
  (if IsHit
    (Utilities|IsValid _returnvalue
      (:Is%20Valid
        (CallFunction|CacheCurrentlyHovered _returnvalue))
      (:Is%20Not%20Valid
        ;[0.1827 0.152 1] We didn't hit anything relevant, but unhover currently hovered object anyway
        (CallFunction|CacheCurrentlyHovered :!label _label)))
    (else
      (goto _label))))

(event Custom|CacheCurrentlyHovered
  (params (incoming :type BP%20Interactable%20Object%20Reference))
  (Utilities|IsValid incoming
    (:Is%20Valid
      (if (!= incoming (Variables|Default|GetCurrentlyHoveredActor))
        (Default|OnSelectorHovered incoming self)
        (Utilities|IsValid (Variables|Default|GetCurrentlyHoveredActor) :!label _label
          (:Is%20Valid
            (Default|OnSelectorUnhovered (Variables|Default|GetCurrentlyHoveredActor) self))
          (:Is%20Not%20Valid
            _))
        (Variables|Default|SetCurrentlyHoveredActor incoming)))
    (:Is%20Not%20Valid
      (goto _label))))

(event Custom|TryInteraction
  (bind (_isvalid _interactable) (CallFunction|GetCurrentlyHoveredActor))
  (if _isvalid
    (Default|Interact _interactable self)))

(event EventBeginPlay
  (if (> (Variables|Sampling|GetSampleRate) 0.0)
    (Utilities|Time|SetTimerbyEvent (EventDispatchers|CreateEvent :!event Custom|PerformSampling) (Variables|Sampling|GetSampleRate) true)))

(fn ConstructionScript)

(fn GetPlayer
  (bind _asik_vr_player (Utilities|Casting|CastToIK_VR_Player (Game|GetPlayerController 0)))
  (return _asik_vr_player))

(fn GetCurrentlyHoveredActor
  (bind _currentlyhoveredactor (Variables|Default|GetCurrentlyHoveredActor))
  (if (Utilities|IsValid (Variables|Default|GetCurrentlyHoveredActor))
    (return true _currentlyhoveredactor (Components|GetOwner _currentlyhoveredactor))
    (else
      (return false 0 0))))