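; BP_MovementSelector is a teleport locomotion selector that shows a target marker and moves the player to the chosen spot.
; Each trace hit counts as valid only if a synchronous navigation path reaches it and the surface slope is under 45 degrees.
; The marker aligns to the hit normal and shows validity through a dynamic material parameter.
; On interaction, the player teleports to the last valid location if the current target is valid.
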(event Custom|ToggleMarker
  (params (Visible :type Boolean) (Valid :type Boolean))
  (Rendering|SetVisibility (Variables|Default|GetMarkerMesh) Visible true)
  (Rendering|Material|SetScalarParameterValue (Variables|Default|GetMarkerMaterialInstance) "IsValid" (Math|Conversions|ToFloat(Boolean) Valid) :!class /Script/Engine.MaterialInstanceDynamic))

(event EventOnTraceHiResultt
  (params (IsHit :type Boolean) (Result :type Hit%20Result%20Structure))
  (bind (_bblockinghit _binitialoverlap _time _location _impactpoint _normal) (Collision|BreakHitResult Result))
  (bind _returnvalue (Class|NavigationSystem|GetNavigationSystem))
  (bind _markermesh (Variables|Default|GetMarkerMesh))
  (if IsHit
    (Utilities|IsValid _returnvalue
      (:Is%20Valid
        (bind _returnvalue_2 (Class|NavigationSystem|FindPathtoLocationSynchronously _returnvalue (Transformation|GetActorLocation) _location (CallFunction|GetPlayer)))
        (bind _output_get (Variables|Default|SetTPPossible (and (Utilities|IsValid _returnvalue_2) (< (Class|KismetMathLibrary|DegAcos (Math|Vector|DotProduct _normal "0, 0,1.000000")) 45.0))))
        (CallFunction|ToggleMarker true _output_get)
        (Transformation|SetWorldLocation _markermesh _location false false)
        (Transformation|SetWorldRotation _markermesh (Math|Rotator|MakeRotfromZ _normal) false false)
        (if (Variables|Default|GetTPPossible)
          (Variables|Default|SetLastLocation _location)))
      (:Is%20Not%20Valid
        (Utilities|FlowControl|DoOnce false
          (:Completed
            (Development|PrintString "Navigation is not valid")))))
    (else
      (CallFunction|ToggleMarker false false))))

(event EventTryInteraction
  (if (Variables|Default|GetTPPossible)
    (Default|Teleportto (CallFunction|GetPlayer) (Variables|Default|GetLastLocation) false)))

(fn ConstructionScript
  (|CallParentFunction)
  (bind _returnvalue (Rendering|Material|CreateDynamicMaterialInstance (Variables|Default|GetMarkerMesh) 0 0 :!class /Script/Engine.PrimitiveComponent))
  (Variables|Default|SetMarkerMaterialInstance _returnvalue))